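; BP_RadioTower02 is a destructible radio tower that takes damage from artillery fire.
; On BeginPlay it fills its health and caches the BP_TankGameMode.
; Radial damage counts only when caused by a BP_ArtyProjectile, and is scaled down before being subtracted from health.
; The scaled amount goes to the game mode's tank UI to update the tower health display, and the tower destroys itself once health runs out.
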(event EventBeginPlay
  ;[0.15 0.15 0.15 0.5] Establece la vida
  (Variables|Default|SetHealth (Variables|Default|GetMaxHealth))
  (bind _asbp_tank_game_mode (Utilities|Casting|CastToBP_TankGameMode (Game|GetGameMode)))
  (Variables|Default|SetTankGameMode _asbp_tank_game_mode))

(event Collision|EventActorBeginOverlap
  (params (OtherActor :type Actor%20Object%20Reference)))

(event EventTick
  (params (DeltaSeconds :type Float%20%28single-precision%29)))

(event Game|Damage|EventRadialDamage
  (params (DamageReceived :type Float%20%28single-precision%29) (DamageType :type Damage%20Type%20Object%20Reference) (Origin :type Vector :default "0, 0, 0") (HitInfo :type Hit%20Result%20Structure%20%28by%20ref%29) (InstigatedBy :type Controller%20Object%20Reference) (DamageCauser :type Actor%20Object%20Reference))
  (bind _returnvalue (/ DamageReceived 1.5))
  (bind _tankgamemode (Variables|Default|GetTankGameMode))
  ;[0.15 0.15 0.15 0.5] Recibe daño del artillero y se autodestruye
  (Utilities|Casting|CastToBP_ArtyProjectile DamageCauser)
  (bind _output_get (Variables|Default|SetHealth (- (Variables|Default|GetHealth) _returnvalue)))
  (Utilities|FlowControl|Sequence
    (:then_0
      (Utilities|IsValid _tankgamemode
        (:Is%20Valid
          (Default|UpdateRadioTowerHealth (Variables|/Game/Blueprints/BP_TankGameMode.BP_TankGameMode_C|GetTankUIRef _tankgamemode) _returnvalue))))
    (:then_1
      (if (<= _output_get 0.0)
        (Actor|DestroyActor)))))

(fn ConstructionScript)