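; Player-controlled tank on Chaos vehicle movement, driven through Enhanced Input, with a cannon and health.
; Tick scrolls track materials from speed or wheel rotation when turning, places the crosshair by tracing from the gun socket, and feeds engine and track audio.
; Firing spawns a projectile with effects, hull torque and recoil, then runs a timed reload shown on the crosshair widget.
; Artillery radial damage updates the health bar and swaps in a wreck at zero.
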(event Custom|TrackAnimation
  ;[0.15 0.15 0.15 0.5] Movimiento de la cinta de las ruedas del tanque
  (if (== (Variables|Default|GetYawValue) 0.0)
    (CallFunction|SetTrackOffset)
    (Rendering|Material|SetScalarParameterValueonMaterials (Variables|Character|GetMesh) "OffsetVRT" (Variables|Default|GetTrackOffset))
    (Rendering|Material|SetScalarParameterValueonMaterials (Variables|Character|GetMesh) "OffsetVLT" (Variables|Default|GetTrackOffset))
    (else
      (CallFunction|TurninPlace 7 "OffsetVRT")
      (CallFunction|TurninPlace 0 "OffsetVLT"))))

(event Custom|UpdateCrosshairPosition
  (bind _mesh (Variables|Character|GetMesh))
  (bind _crosshair (Variables|Default|GetCrosshair))
  (bind _returnvalue (Transformation|GetSocketLocation _mesh "gun_1_jntSocket"))
  ;[0.15 0.15 0.15 0.5] Establece la posición de la mira dependiendo de la posición de la camara
  (bind _outactors (Actor|GetAllActorsOfClass "/Game/Tank/Blueprints/BP_TankProjectile.BP_TankProjectile_C"))
  (bind _outhit (Collision|LineTraceByChannel _returnvalue (+ _returnvalue (* (Math|Vector|GetForwardVector (Transformation|GetSocketRotation _mesh "gun_1_jntSocket")) 1e+06)) "TraceTypeQuery1" false _outactors "None"))
  (if (.bBlockingHit (Collision|BreakHitResult _outhit))
    (Transformation|SetWorldLocation _crosshair (.ImpactPoint (Collision|BreakHitResult _outhit)) false false)
    (else
      (Transformation|SetWorldLocation _crosshair (.TraceEnd (Collision|BreakHitResult _outhit)) false false))))

(event Custom|CanShootAgain
  ;[0.15 0.15 0.15 0.5] Disparo de proyectil desde el Tanque
  (Variables|Default|SetCanShoot true))

(event Custom|SoundManagement
  (bind _chaoswheeledvehiclemovement (Variables|Default|GetChaosWheeledVehicleMovement))
  ;[0.15 0.15 0.15 0.5] Gestiona el donido del motor y el sonio de las ruedas
  (Audio|Parameter|SetFloatParameter (Variables|Default|GetEngine) "RPM" (Class|ChaosWheeledVehicleMovementComponent|GetEngineRotationSpeed _chaoswheeledvehiclemovement) :!class /Script/Engine.AudioComponent)
  (Audio|Parameter|SetFloatParameter (Variables|Default|GetTrack) "Speed" (Math|Float|Absolute(Float) (Class|ChaosVehicleMovementComponent|GetForwardSpeedMPH _chaoswheeledvehiclemovement)) :!class /Script/Engine.AudioComponent))

(event Input|EnhancedActionEvents|EnhancedInputActionIA_LookUpDown
  (params (ActionValue :type Float%20%28double-precision%29) (ElapsedSeconds :type Float%20%28double-precision%29) (TriggeredSeconds :type Float%20%28double-precision%29) (InputAction :type Input%20Action%20Object%20Reference :default "/Game/Tank/Input/IA_LookUpDown.IA_LookUpDown"))
  ;[0.15 0.15 0.15 0.5] Movimiento de camara en el eje Y
  (Pawn|Input|AddControllerPitchInput (* ActionValue -1.0)))

(event Input|EnhancedActionEvents|EnhancedInputActionIA_LeftRight
  (params (ActionValue :type Float%20%28double-precision%29) (ElapsedSeconds :type Float%20%28double-precision%29) (TriggeredSeconds :type Float%20%28double-precision%29) (InputAction :type Input%20Action%20Object%20Reference :default "/Game/Tank/Input/IA_LeftRight.IA_LeftRight"))
  ;[0.15 0.15 0.15 0.5] Movimiento de camara en el eje X
  (Pawn|Input|AddControllerYawInput ActionValue))

(event Input|EnhancedActionEvents|EnhancedInputActionIA_Forward
  (params (ActionValue :type Float%20%28double-precision%29) (ElapsedSeconds :type Float%20%28double-precision%29) (TriggeredSeconds :type Float%20%28double-precision%29) (InputAction :type Input%20Action%20Object%20Reference :default "/Game/Tank/Input/IA_Forward.IA_Forward"))
  (bind _chaoswheeledvehiclemovement (Variables|Default|GetChaosWheeledVehicleMovement))
  ;[0.15 0.15 0.15 0.5] Movimiento hacia adelante
  (:Triggered
    (Class|ChaosVehicleMovementComponent|SetThrottleInput _chaoswheeledvehiclemovement ActionValue))
  (:Completed
    (Class|ChaosVehicleMovementComponent|SetThrottleInput _chaoswheeledvehiclemovement 0.0)))

(event Input|EnhancedActionEvents|EnhancedInputActionIA_Backward
  (params (ActionValue :type Float%20%28double-precision%29) (ElapsedSeconds :type Float%20%28double-precision%29) (TriggeredSeconds :type Float%20%28double-precision%29) (InputAction :type Input%20Action%20Object%20Reference :default "/Game/Tank/Input/IA_Backward.IA_Backward"))
  (bind _chaoswheeledvehiclemovement (Variables|Default|GetChaosWheeledVehicleMovement))
  ;[0.15 0.15 0.15 0.5] Movimiento hacia atras
  (:Triggered
    (Class|ChaosVehicleMovementComponent|SetBrakeInput _chaoswheeledvehiclemovement ActionValue))
  (:Completed
    (Class|ChaosVehicleMovementComponent|SetBrakeInput _chaoswheeledvehiclemovement 0.0)))

(event Input|EnhancedActionEvents|EnhancedInputActionIA_GoLeftRight
  (params (ActionValue :type Float%20%28double-precision%29) (ElapsedSeconds :type Float%20%28double-precision%29) (TriggeredSeconds :type Float%20%28double-precision%29) (InputAction :type Input%20Action%20Object%20Reference :default "/Game/Tank/Input/IA_GoLeftRight.IA_GoLeftRight"))
  (bind _chaoswheeledvehiclemovement (Variables|Default|GetChaosWheeledVehicleMovement))
  ;[0.15 0.15 0.15 0.5] Girar a la derecha e izquierda
  (:Triggered
    (bind _output_get (Variables|Default|SetYawValue ActionValue))
    (Class|ChaosVehicleMovementComponent|SetYawInput _chaoswheeledvehiclemovement _output_get))
  (:Completed
    (Class|ChaosVehicleMovementComponent|SetYawInput _chaoswheeledvehiclemovement 0.0)))

(event Input|EnhancedActionEvents|EnhancedInputActionIA_Handbrake
  (params (ActionValue :type Boolean) (ElapsedSeconds :type Float%20%28double-precision%29) (TriggeredSeconds :type Float%20%28double-precision%29) (InputAction :type Input%20Action%20Object%20Reference :default "/Game/Tank/Input/IA_Handbrake.IA_Handbrake"))
  (bind _chaoswheeledvehiclemovement (Variables|Default|GetChaosWheeledVehicleMovement))
  ;[0.15 0.15 0.15 0.5] Freno de mano del tanque
  (:Started
    (Class|ChaosVehicleMovementComponent|SetHandbrakeInput _chaoswheeledvehiclemovement true))
  (:Completed
    (Class|ChaosVehicleMovementComponent|SetHandbrakeInput _chaoswheeledvehiclemovement false)))

(event Input|EnhancedActionEvents|EnhancedInputActionIA_Fire
  (params (ActionValue :type Boolean) (ElapsedSeconds :type Float%20%28double-precision%29) (TriggeredSeconds :type Float%20%28double-precision%29) (InputAction :type Input%20Action%20Object%20Reference :default "/Game/Tank/Input/IA_Fire.IA_Fire"))
  (bind _mesh (Variables|Character|GetMesh))
  (bind _mesh_2 (Variables|Character|GetMesh))
  (bind _returnvalue (Transformation|GetSocketTransform _mesh "gun_1_jntSocket" "RTS_World"))
  (bind (_location _rotation) (Math|Transform|BreakTransform _returnvalue))
  ;[0.15 0.15 0.15 0.5] Disparo de proyectil desde el Tanque
  (:Started
    (if (Variables|Default|GetCanShoot)
      (Game|SpawnActorfromClass "/Game/Tank/Blueprints/BP_TankProjectile.BP_TankProjectile_C" _returnvalue "Undefined" "MultiplyWithRoot" 0 0)
      (Niagara|SpawnSystemAttached "/Game/Tank/Assets/Vehicles/East_Tank_T72b/FX/NS_East_Tank_T72B.NS_East_Tank_T72B" (Variables|Character|GetMesh) "gun_1_jntSocket" _location _rotation "KeepWorldPosition" false)
      (Audio|SpawnSoundatLocation "/Game/Tank/Assets/Sounds/ES_Cannon_Fire_Single_-_SFX_Producer.ES_Cannon_Fire_Single_-_SFX_Producer" (Transformation|GetActorLocation) "0, 0, 0" 1.0 1.0 0.0 0 0)
      (Class|PrimitiveComponent|AddTorqueinRadians _mesh_2 (Math|Transform|TransformDirection (Transformation|GetSocketTransform _mesh_2 "turret_jnt" "RTS_World") "0.000000,-25.000000,0.000000") "cog_jnt" true)
      (Variables|Default|SetCanShoot false)
      (Utilities|Time|SetTimerbyEvent (delegate Custom|CanShootAgain) 2.0)
      (Utilities|FlowControl|Sequence
        (:then_0
          (bind _recoilvalue (Timeline|Recoil PlayFromStart)
            (:Update
              (Variables|Default|SetRecoil%20Value _recoilvalue))))
        (:then_1
          (bind _reloadvalue (Timeline|Reload PlayFromStart)
            (:Update
              (Class|BPICrosshairInterface|SetReloadProgressBar(Message) (UserInterface|GetUserWidgetObject (Variables|Default|GetCrosshair)) _reloadvalue))))))))

(event EventBeginPlay
  (bind _returnvalue (Game|GetPlayerController 0))
  ;[0.15 0.15 0.15 0.5] Configura el Input Mapping Context
  (Input|AddMappingContext (PlayerController|LocalPlayerSubsystems|GetEnhancedInputLocalPlayerSubsystem _returnvalue) "/Game/Tank/Input/IMC_Tank.IMC_Tank" 0 "(bIgnoreAllPressedKeysUntilRelease=True,bForceImmediately=False,bNotifyUserSettings=False)")
  (bind _returnvalue_2 (UserInterface|CreateWidget "/Game/Tank/Widgets/WBP_TankUI.WBP_TankUI_C"))
  (UserInterface|Viewport|AddtoViewport _returnvalue_2 0)
  (Variables|/Script/Engine.PlayerController|SetbShowMouseCursor _returnvalue false)
  (Input|SetInputModeGameOnly _returnvalue false)
  (CallFunction|AddHealth (Variables|Default|GetMaxHealth)))

(event Collision|EventActorBeginOverlap
  (params (OtherActor :type Actor%20Object%20Reference)))

(event EventTick
  (params (DeltaSeconds :type Float%20%28single-precision%29))
  (CallFunction|TrackAnimation)
  (CallFunction|UpdateCrosshairPosition)
  (CallFunction|SoundManagement))

(event Game|Damage|EventRadialDamage
  (params (DamageReceived :type Float%20%28single-precision%29) (DamageType :type Damage%20Type%20Object%20Reference) (Origin :type Vector :default "0, 0, 0") (HitInfo :type Hit%20Result%20Structure%20%28by%20ref%29) (InstigatedBy :type Controller%20Object%20Reference) (DamageCauser :type Actor%20Object%20Reference))
  ;[0.15 0.15 0.15 0.5] Recibe daño del Artillero
  (Utilities|Casting|CastToBP_ArtyProjectile DamageCauser)
  (bind _output_get (Variables|Default|SetHealth (- (Variables|Default|GetHealth) DamageReceived)))
  (CallFunction|UpdateHealthBar)
  (if (<= _output_get 0.0)
    (Game|SpawnActorfromClass "/Game/Tank/Blueprints/BP_DamagedTank.BP_DamagedTank_C" (Transformation|GetActorTransform) "Undefined" "MultiplyWithRoot" 0 0)
    (Actor|DestroyActor)))

(fn ConstructionScript)

(fn TurninPlace
  (params (WheelIndex :type Integer) (ParamMaterialName :type Name))
  (Rendering|Material|SetScalarParameterValueonMaterials (Variables|Character|GetMesh) ParamMaterialName (* (Class|ChaosVehicleWheel|GetRotationAngle (Utilities|Array|Get(acopy) (Variables|/Script/ChaosVehicles.ChaosWheeledVehicleMovementComponent|GetWheels (Variables|Default|GetChaosWheeledVehicleMovement)) WheelIndex)) 0.0035)))

(fn SetTrackOffset
  (Variables|Default|SetTrackOffset (+ (Math|Float|MapRangeClamped (Class|ChaosVehicleMovementComponent|GetForwardSpeedMPH (Variables|Default|GetChaosWheeledVehicleMovement)) -7e+01 7e+01 0.4 -0.4) (Variables|Default|GetTrackOffset))))

(fn UpdateHealthBar
  (Class|BPICrosshairInterface|UpdateHealth(Message) (UserInterface|GetUserWidgetObject (Variables|Default|GetCrosshair)) (/ (Variables|Default|GetHealth) (Variables|Default|GetMaxHealth))))

(fn AddHealth
  (params (HealthAmount :type Float%20%28double-precision%29))
  (Variables|Default|SetHealth (Math|Float|Clamp(Float) (+ HealthAmount (Variables|Default|GetHealth)) 0.0 (Variables|Default|GetMaxHealth)))
  (CallFunction|UpdateHealthBar))