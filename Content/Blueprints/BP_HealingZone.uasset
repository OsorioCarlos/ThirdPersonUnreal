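; BP_HealingZone is an area that periodically restores health to a tank while it stays inside.
; When a BP_Tank enters HealingArea, the zone stores it and starts a looping timer that calls HealPlayer at HealingInterval, adding HealingAmount through AddHealth.
; Leaving clears the timer and the stored tank.
; It tracks a single tank and timer handle, so it handles one occupant at a time.
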(event OnComponentBeginOverlap(HealingArea)
  (params (OverlappedComponent :type Primitive%20Component%20Object%20Reference) (OtherActor :type Actor%20Object%20Reference) (OtherComp :type Primitive%20Component%20Object%20Reference) (OtherBodyIndex :type Integer) (bFromSweep :type Boolean) (SweepResult :type Hit%20Result%20Structure%20%28by%20ref%29))
  (bind _asbp_tank (Utilities|Casting|CastToBP_Tank OtherActor))
  (Variables|Default|SetPlayer _asbp_tank)
  (bind _returnvalue (Utilities|Time|SetTimerbyFunctionName 0 "HealPlayer" (Variables|Default|GetHealingInterval) true))
  (Variables|Default|SetHealingTimer _returnvalue))

(event OnComponentEndOverlap(HealingArea)
  (params (OverlappedComponent :type Primitive%20Component%20Object%20Reference) (OtherActor :type Actor%20Object%20Reference) (OtherComp :type Primitive%20Component%20Object%20Reference) (OtherBodyIndex :type Integer))
  (Utilities|Casting|CastToBP_Tank OtherActor)
  (Utilities|Time|ClearandInvalidateTimerbyHandle (Variables|Default|GetHealingTimer))
  (Variables|Default|SetPlayer 0))

(event EventBeginPlay)

(event Collision|EventActorBeginOverlap
  (params (OtherActor :type Actor%20Object%20Reference)))

(event EventTick
  (params (DeltaSeconds :type Float%20%28single-precision%29)))

(fn ConstructionScript)

(fn HealPlayer
  (bind _player (Variables|Default|GetPlayer))
  (Utilities|IsValid _player
    (:Is%20Valid
      (Default|AddHealth _player (Variables|Default|GetHealingAmount)))))