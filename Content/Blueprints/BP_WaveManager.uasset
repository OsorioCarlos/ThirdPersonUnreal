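; Wave manager for the tank game that spawns escalating waves of BP_Arty enemies.
; On BeginPlay it registers with BP_TankGameMode and starts a wave, raising the wave number and enemy count, then spawning at random X/Y points drawn from SpawnZones boxes.
; Increase/decrease events track active enemies and update the tank UI.
; Tick polls for zero enemies, then after a Delay destroys all BP_DamagedArty actors and starts the next wave.
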(event Custom|IncreaseActiveEnemies
  (Variables|Default|SetActiveEnemies (+ (Variables|Default|GetActiveEnemies) 1))
  (CallFunction|UpdateEnemiesCounter))

(event Custom|DecreaseActiveEnemies
  (Variables|Default|SetActiveEnemies (- (Variables|Default|GetActiveEnemies) 1))
  (CallFunction|UpdateEnemiesCounter))

(event EventBeginPlay
  ;[0.15 0.15 0.15 0.5] Guarda la referencia del WaveManager en TankGameMode y Spawnea enemigos
  (bind _asbp_tank_game_mode (Utilities|Casting|CastToBP_TankGameMode (Game|GetGameMode)))
  (Variables|/Game/Blueprints/BP_TankGameMode.BP_TankGameMode_C|SetWaveManagerRef _asbp_tank_game_mode self)
  (CallFunction|StartWave))

(event Collision|EventActorBeginOverlap
  (params (OtherActor :type Actor%20Object%20Reference)))

(event EventTick
  (params (DeltaSeconds :type Float%20%28single-precision%29))
  ;[0.15 0.15 0.15 0.5] Verifica si todos los enemigos han sido derrotados y comienza una nueva oleda
  (if (== (Variables|Default|GetActiveEnemies) 0)
    (Utilities|FlowControl|Delay 1e+01)
    (bind _outactors (Actor|GetAllActorsOfClass "/Game/Arty/Blueprints/BP_DamagedArty.BP_DamagedArty_C"))
    (for _array_element _outactors
      (Actor|DestroyActor _array_element))
    (CallFunction|StartWave)))

(fn ConstructionScript)

(fn SpawnEnemies
  (bind _spawnzones (Variables|Default|GetSpawnZones))
  (bind _returnvalue (Utilities|Array|Length _spawnzones))
  (bind _returnvalue_2 (- _returnvalue 1))
  (bind _returnvalue_3 (Math|Random|RandomIntegerinRange 0 _returnvalue_2))
  (bind _output (Utilities|Array|Get(acopy) _spawnzones _returnvalue_3))
  (bind _boxzone (Variables|/Game/Blueprints/BP_SpawnZone.BP_SpawnZone_C|GetBoxZone _output))
  (bind _returnvalue_4 (Components|Box|GetScaledBoxExtent _boxzone))
  (bind _returnvalue_5 (Transformation|GetWorldLocation _boxzone))
  (bind _returnvalue_6 (Math|Random|RandomPointinBoundingBox _returnvalue_5 _returnvalue_4))
  (bind (_x _y) (Math|Vector|BreakVector _returnvalue_6))
  (for _index (range 0 (- (Variables|Default|GetEnemiesToSpawn) 1))
    (Game|SpawnActorfromClass "/Game/Arty/Blueprints/BP_Arty.BP_Arty_C" (Math|Transform|MakeTransform (Math|Vector|MakeVector _x _y 0.0)) "Undefined" "MultiplyWithRoot" 0 0)
    (CallFunction|IncreaseActiveEnemies)))

(fn StartWave
  (bind _output_get (Variables|Default|SetWaveNumber (+ (Variables|Default|GetWaveNumber) 1)))
  (bind _asbp_tank_game_mode (Utilities|Casting|CastToBP_TankGameMode (Game|GetGameMode)))
  (Default|UpdateWavesCounter (Variables|/Game/Blueprints/BP_TankGameMode.BP_TankGameMode_C|GetTankUIRef _asbp_tank_game_mode) _output_get)
  (Variables|Default|SetEnemiesToSpawn (+ (Variables|Default|GetEnemiesToSpawn) 5))
  (CallFunction|SpawnEnemies))

(fn UpdateEnemiesCounter
  (bind _asbp_tank_game_mode (Utilities|Casting|CastToBP_TankGameMode (Game|GetGameMode)))
  (Default|UpdateEnemiesCounter (Variables|/Game/Blueprints/BP_TankGameMode.BP_TankGameMode_C|GetTankUIRef _asbp_tank_game_mode) (Variables|Default|GetActiveEnemies)))