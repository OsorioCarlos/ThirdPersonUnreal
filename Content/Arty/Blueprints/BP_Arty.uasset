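; Enemy artillery piece that shells the player tank or RadioTower-tagged actors, preferring the player, within a set distance band.
; A looping timer spawns a projectile aimed at the target, with effects, sound and a recoil timeline.
; Tick derives YawValue from a moving-target velocity prediction.
; Radial damage from a tank projectile swaps it for a damaged actor and decrements the wave manager's active enemy count.
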(event Custom|Fire
  ;[0.15 0.15 0.15 0.5] Disparo al jugador
  (bind _actor (CallFunction|GetTarget))
  (Utilities|IsValid _actor
    (:Is%20Valid
      (CallFunction|FireTarget _actor)
      (bind _recoilvalue (Timeline|Recoil Play)
        (:Update
          (Variables|Default|SetRecoilValue _recoilvalue))))))

(event EventBeginPlay
  ;[0.15 0.15 0.15 0.5] Guarda  la referencia al jugador
  (Utilities|FlowControl|Sequence
    (:then_0
      (bind _outactors (Actor|GetAllActorswithTag "RadioTower"))
      (Variables|Default|SetRadioTowers _outactors))
    (:then_1
      (bind _asbp_tank (Utilities|Casting|CastToBP_Tank (Game|Player|GetPlayerPawn 0)))
      (Variables|Default|SetPlayer _asbp_tank))
    (:then_2
      (Utilities|Time|SetTimerbyEvent (delegate Custom|Fire) 5.0 true))))

(event Collision|EventActorBeginOverlap
  (params (OtherActor :type Actor%20Object%20Reference)))

(event EventTick
  (params (DeltaSeconds :type Float%20%28single-precision%29))
  ;[0.15 0.15 0.15 0.5] Predice el movimiento del jugador
  (bind _actor (CallFunction|GetTarget))
  (Utilities|IsValid _actor
    (:Is%20Valid
      (bind _outlaunchvelocity (Class|GameplayStatics|SuggestProjectileVelocityMovingTarget (Transformation|GetSocketLocation (Variables|Default|GetSkeletalMesh) "gun_jntSocket") _actor "0, 0, 0" 0.0 1.0 "None"))
      (Variables|Default|SetYawValue (.yaw (Math|Rotator|Delta(Rotator) (Math|Rotator|MakeRotfromX _outlaunchvelocity) (Transformation|GetActorRotation)))))))

(event Game|Damage|EventRadialDamage
  (params (DamageReceived :type Float%20%28single-precision%29) (DamageType :type Damage%20Type%20Object%20Reference) (Origin :type Vector :default "0, 0, 0") (HitInfo :type Hit%20Result%20Structure%20%28by%20ref%29) (InstigatedBy :type Controller%20Object%20Reference) (DamageCauser :type Actor%20Object%20Reference))
  ;[0.15 0.15 0.15 0.5] Recibe daño del jugador y se autodestruye
  (Utilities|Casting|CastToBP_TankProjectile DamageCauser)
  (Game|SpawnActorfromClass "/Game/Arty/Blueprints/BP_DamagedArty.BP_DamagedArty_C" (Transformation|GetActorTransform) "Undefined" "MultiplyWithRoot" 0 0)
  (bind _asbp_tank_game_mode (Utilities|Casting|CastToBP_TankGameMode (Game|GetGameMode)))
  (Default|DecreaseActiveEnemies (Variables|/Game/Blueprints/BP_TankGameMode.BP_TankGameMode_C|GetWaveManagerRef _asbp_tank_game_mode))
  (Actor|DestroyActor))

(fn ConstructionScript)

(fn FireTarget
  (params (BP_Target :type Actor%20Object%20Reference))
  (bind _skeletalmesh (Variables|Default|GetSkeletalMesh))
  (bind _returnvalue (Transformation|GetSocketTransform _skeletalmesh "gun_jntSocket" "RTS_World"))
  (Game|SpawnActorfromClass "/Game/Arty/Blueprints/BP_ArtyProjectile.BP_ArtyProjectile_C" (Transformation|GetSocketTransform _skeletalmesh "gun_jntSocket" "RTS_World") "Undefined" "MultiplyWithRoot" 0 BP_Target 0)
  (Effects|SpawnEmitteratLocation "/Game/Arty/Assets/Vehicles/West_Arty_M777/FX/PS_CannonShockwave_01_West_Arty_M777.PS_CannonShockwave_01_West_Arty_M777" (Transformation|GetSocketLocation _skeletalmesh "cog_jntSocket"))
  (Effects|SpawnEmitterAttached "/Game/Arty/Assets/Vehicles/West_Arty_M777/FX/PS_CannonExplosion_01_West_Arty_M777.PS_CannonExplosion_01_West_Arty_M777" _skeletalmesh "gun_jntSocket" (.location _returnvalue) (.rotation _returnvalue) "1.000000,1.000000,1.000000" "KeepWorldPosition")
  (Audio|SpawnSoundatLocation "/Game/Tank/Assets/Sounds/ES_Cannon_Fire_Single_-_SFX_Producer.ES_Cannon_Fire_Single_-_SFX_Producer" (.location _returnvalue) "0, 0, 0" 1.0 1.0 0.0 0 0))

(fn CanFireTarget
  (params (BP_Target :type Actor%20Object%20Reference))
  (Utilities|IsValid BP_Target
    (:Is%20Valid
      (return (Math|Float|InRange(Float) (Math|Vector|Distance(Vector) (Transformation|GetActorLocation BP_Target) (Transformation|GetActorLocation)) 3.5e+03 1e+04)))
    (:Is%20Not%20Valid
      (return false))))

(fn GetTarget
  (bind _player (Variables|Default|GetPlayer))
  (bind _value (CallFunction|CanFireTarget _player))
  (if _value
    (return _player)
    (else
      (for _array_element (Variables|Default|GetRadioTowers)
        (bind _value_2 (CallFunction|CanFireTarget _array_element))
        (if _value_2
          (return _array_element)))
      (return 0))))