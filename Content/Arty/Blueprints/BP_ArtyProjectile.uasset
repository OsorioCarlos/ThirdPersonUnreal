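; BP_ArtyProjectile is an artillery shell that launches toward a target and explodes where it stops.
; On BeginPlay, if Target is valid, it sets its ProjectileMovement velocity using SuggestProjectileVelocityMovingTarget, which leads a moving target over a fixed flight time.
; When the projectile stops, it applies radial damage with falloff, spawns a Niagara dust explosion and sound at the impact point, then destroys itself.
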(event OnProjectileStop(ProjectileMovement)
  (params (ImpactResult :type Hit%20Result%20Structure%20%28by%20ref%29))
  (bind _location (Collision|BreakHitResult ImpactResult))
  (bind _self self)
  ;[0.15 0.15 0.15 0.5] Provoca daño en área
  (Class|GameplayStatics|ApplyRadialDamagewithFalloff 25.0 1e+01 _location 1e+02 5e+02 1.0 0 (Utilities|Array|MakeArray _self) _self 0 "ECC_Visibility")
  (Niagara|SpawnSystematLocation "/Game/Tank/Assets/VigilanteContent/MsvFx_Niagara_Explosion_Pack_01/Prefabs/Niagara_Dust_Explosion_01.Niagara_Dust_Explosion_01" _location (Math|Rotator|MakeRotfromX _location))
  (Audio|SpawnSoundatLocation "/Game/Tank/Assets/Sounds/ES_Grenade_Explosion_14_-_SFX_Producer.ES_Grenade_Explosion_14_-_SFX_Producer" _location "0, 0, 0" 1.0 1.0 0.0 "/Game/Tank/Sounds/SA_Explosion.SA_Explosion" 0)
  (Actor|DestroyActor))

(event EventBeginPlay
  (bind _target (Variables|Default|GetTarget))
  (Utilities|IsValid _target
    (:Is%20Valid
      (bind _outlaunchvelocity (Class|GameplayStatics|SuggestProjectileVelocityMovingTarget (Transformation|GetActorLocation) _target "0, 0, 0" 0.0 4.0 "None"))
      (Variables|/Script/Engine.MovementComponent|SetVelocity (Variables|Default|GetProjectileMovement) _outlaunchvelocity))))

(event Collision|EventActorBeginOverlap
  (params (OtherActor :type Actor%20Object%20Reference)))

(event EventTick
  (params (DeltaSeconds :type Float%20%28single-precision%29)))

(fn ConstructionScript)